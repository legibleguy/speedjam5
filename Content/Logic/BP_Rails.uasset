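; Spline rail that catches a physics-simulating actor, apparently a train, carries it along the track and launches it at the end.
; Construction builds spline meshes between points and orients a debug direction component.
; A trigger overlap or preset target starts a physics handle grab, with a timeline moving it along the spline using an up offset and corrected rotation.
; On finish it releases the target with a forward velocity impulse, never clearing the target.
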(event OnComponentBeginOverlap(GrabTrigger)
  (params (OverlappedComponent :type Primitive%20Component%20Object%20Reference) (OtherActor :type Actor%20Object%20Reference) (OtherComp :type Primitive%20Component%20Object%20Reference) (OtherBodyIndex :type Integer) (bFromSweep :type Boolean) (SweepResult :type Hit%20Result%20Structure%20%28by%20ref%29))
  (Utilities|IsValid (Variables|Default|GetCurrTargetActor)
    (:Is%20Not%20Valid
      (bind _asprimitive_component (Utilities|Casting|CastToPrimitiveComponent (Variables|/Script/Engine.Actor|GetRootComponent OtherActor)))
      (if (Physics|IsSimulatingPhysics _asprimitive_component "None")
        (Variables|Default|SetCurrTargetActor OtherActor)
        (Utilities|FlowControl|Delay 1.0)
        (CallFunction|InitGrab)
        (Utilities|FlowControl|Delay 2.0)
        (bind _progress (Timeline|TakeOffTimeline PlayFromStart)
          (:Update
            (Variables|Default|SetCurrentGrabTime _progress)
            (Class|PhysicsHandleComponent|SetTargetLocationandRotation (Variables|Default|GetPhysicsHandle) (CallFunction|CurrentGrabLocation) (CallFunction|CurrentGrabRotation)))
          (:Finished
            (Physics|Components|PhysicsHandle|ReleaseComponent (Variables|Default|GetPhysicsHandle))
            (Physics|AddImpulse (.AsPrimitive%20Component (Utilities|Casting|CastToPrimitiveComponent (Variables|/Script/Engine.Actor|GetRootComponent (Variables|Default|GetCurrTargetActor)))) (* (CallFunction|TryGetTrainForwardVector (Variables|Default|GetCurrTargetActor)) (Variables|Default|GetTakeOffReleasePower)) "None" true)))))))

(event EventBeginPlay
  (Utilities|IsValid (Variables|Default|GetCurrTargetActor)
    (:Is%20Valid
      (CallFunction|InitGrab)
      (Utilities|FlowControl|Delay 2.0)
      (bind _progress (Timeline|TakeOffTimeline PlayFromStart)
        (:Update
          (Variables|Default|SetCurrentGrabTime _progress)
          (Class|PhysicsHandleComponent|SetTargetLocationandRotation (Variables|Default|GetPhysicsHandle) (CallFunction|CurrentGrabLocation) (CallFunction|CurrentGrabRotation)))
        (:Finished
          (Physics|Components|PhysicsHandle|ReleaseComponent (Variables|Default|GetPhysicsHandle))
          (Physics|AddImpulse (.AsPrimitive%20Component (Utilities|Casting|CastToPrimitiveComponent (Variables|/Script/Engine.Actor|GetRootComponent (Variables|Default|GetCurrTargetActor)))) (* (CallFunction|TryGetTrainForwardVector (Variables|Default|GetCurrTargetActor)) (Variables|Default|GetTakeOffReleasePower)) "None" true))))))

(event Collision|EventActorBeginOverlap
  (params (OtherActor :type Actor%20Object%20Reference)))

(event EventTick
  (params (DeltaSeconds :type Float%20%28single-precision%29)))

(fn ConstructionScript
  (Utilities|FlowControl|Sequence
    (:then_0
      (for _index (range 0 (- (Spline|GetNumberOfSplinePoints (Variables|Default|GetSpline)) 1))
        (LocalVariables|SetCurrPoint _index)
        (bind _returnvalue (AddComponent|AddSplineMeshComponent false))
        (LocalVariables|SetNewMesh _returnvalue)
        (SplineMesh|SetStartandEnd (LocalVariables|GetNewMesh) (Spline|GetLocationatSplinePoint (Variables|Default|GetSpline) (LocalVariables|GetCurrPoint) "Local") (Spline|GetTangentatSplinePoint (Variables|Default|GetSpline) (LocalVariables|GetCurrPoint) "Local") (Spline|GetLocationatSplinePoint (Variables|Default|GetSpline) (+ (LocalVariables|GetCurrPoint) 1) "Local") (Spline|GetTangentatSplinePoint (Variables|Default|GetSpline) (+ (LocalVariables|GetCurrPoint) 1) "Local") true :!class /Script/Engine.SplineMeshComponent)))
    (:then_1
      (Transformation|SetWorldRotation (Variables|Default|GetDebugDirection) (CallFunction|CurrentGrabRotation) false false))
    (:then_2
      (bind _outactors (Actor|GetAllActorsOfClass "/Game/Logic/BP_Train.BP_Train_C")))))

(fn InitGrab
  (bind _asprimitive_component (Utilities|Casting|CastToPrimitiveComponent (Variables|/Script/Engine.Actor|GetRootComponent (Variables|Default|GetCurrTargetActor))))
  (bind _output_get (LocalVariables|SetTargetComponent _asprimitive_component))
  (if (Physics|IsSimulatingPhysics _output_get "None")
    (Physics|Components|PhysicsHandle|GrabComponentatLocationwithRotation (Variables|Default|GetPhysicsHandle) (LocalVariables|GetTargetComponent) "None" (CallFunction|CurrentGrabLocation) (CallFunction|CurrentGrabRotation))))

(fn CurrentGrabLocation
  (return (+ (Spline|GetLocationatTime (Variables|Default|GetSpline) (Variables|Default|GetCurrentGrabTime) "World" true) (* (Class|SplineComponent|GetUpVectoratTime (Variables|Default|GetSpline) (Variables|Default|GetCurrentGrabTime) "World" true) (Variables|Default|GetGrabUpOffset)))))

(fn CurrentGrabRotation
  (bind _outdefault (CallFunction|GetDefaultTrainRotation))
  (bind _spline (Variables|Default|GetSpline))
  (bind _currentgrabtime (Variables|Default|GetCurrentGrabTime))
  (bind _returnvalue (Class|SplineComponent|GetRotationatTime _spline _currentgrabtime "World" true))
  (bind _returnvalue_2 (Math|Transform|MakeTransform "0, 0, 0" _returnvalue))
  (bind _returnvalue_3 (Math|Transform|InverseTransformRotation _returnvalue_2 _outdefault))
  (return (Math|Rotator|MakeRotator (* (.pitch _returnvalue_3) 1.0) (+ (* (.yaw _returnvalue_3) -1.0) 1.8e+02) (* (.roll _returnvalue_3) -1.0))))