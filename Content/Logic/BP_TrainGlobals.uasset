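; BP_TrainGlobals is a set of shared train helper functions for default rotation and forward direction.
; GetDefaultTrainRotation returns a fixed rotation.
; TryGetTrainForwardVector asks actors implementing BP_TrainInterface for their forward vector through an interface message and falls back to the actor's own forward vector otherwise.
; An invalid input yields a zero vector.
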(fn GetDefaultTrainRotation
  (return "-90.000000,180.000000,90.000000"))

(fn TryGetTrainForwardVector
  (params (MaybeTrain :type Actor%20Object%20Reference))
  (Utilities|IsValid MaybeTrain
    (:Is%20Valid
      (if (Utilities|DoesObjectImplementInterface MaybeTrain "/Game/Logic/BP_TrainInterface.BP_TrainInterface_C")
        (bind _outforward (Class|BPTrainInterface|RequestTrainForwardVector(Message) MaybeTrain))
        (return _outforward)
        (else
          (return (Transformation|GetActorForwardVector MaybeTrain)))))
    (:Is%20Not%20Valid
      (return "0, 0, 0"))))